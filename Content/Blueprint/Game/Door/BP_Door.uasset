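; Key-gated room door that streams the level as the player progresses, with the ID 4 trigger starting the photography ending instead.
; It counts matching BP_Key actors and shows progress until unlocked; EventOpen then swings it via Timeline and calls the next BP_RoomManager room.
; Trigger overlaps close the door behind the player, destroying the previous non-clone room on the new-room side.
; ID parity mirrors initial rotation and trigger placement.
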(event OnComponentBeginOverlap(Trigger)
  (params (OverlappedComponent :type Primitive%20Component%20Object%20Reference) (OtherActor :type Actor%20Object%20Reference) (OtherComp :type Primitive%20Component%20Object%20Reference) (OtherBodyIndex :type Integer) (bFromSweep :type Boolean) (SweepResult :type Hit%20Result%20Structure%20%28by%20ref%29))
  (bind _asbp_player (Utilities|Casting|CastToBP_Player OtherActor))
  (if (== (Variables|Default|GetID) 4)
    (CallFunction|END)
    (else
      (CallFunction|NormalDoor _asbp_player))))

(event Custom|Position
  (if (Variables|NewRoom|GetUp?)
    (Variables|NewRoom|SetDoorPosition 1.0)
    (else
      (Variables|NewRoom|SetDoorPosition -1.0))))

(event Custom|Start
  (if (not (== (Variables|Default|GetID) 1))
    (Variables|NewRoom|SetNewRoom true)
    (Variables|NewRoom|SetNewDoor true)
    (if (not (> (Math|Integer|%(Integer) (Variables|Default|GetID) 2) 0))
      (Variables|NewRoom|SetUp? true))))

(event Custom|FixDoor
  (bind _returnvalue (Transformation|GetActorRotation))
  (bind _trigger (Variables|Default|GetTrigger))
  (bind _trigger_2 (Variables|Default|GetTrigger))
  (bind (_roll _pitch _yaw) (Math|Rotator|BreakRotator _returnvalue))
  (bind _relativelocation (Variables|/Script/Engine.SceneComponent|GetRelativeLocation _trigger_2))
  (bind _relativelocation_2 (Variables|/Script/Engine.SceneComponent|GetRelativeLocation _trigger))
  (if (Variables|NewRoom|GetNewRoom)
    (Transformation|SetRelativeRotation (Variables|Default|GetStaticMesh) (Math|Rotator|MakeRotator _roll _pitch (+ _yaw (* 9e+01 (Variables|NewRoom|GetDoorPosition)))) false false)
    (if (Variables|NewRoom|GetUp?)
      (Transformation|SetRelativeLocation (Variables|Default|GetTrigger) (Math|Vector|MakeVector (* (* (.x _relativelocation) (Variables|NewRoom|GetDoorPosition)) -1.0) (.y _relativelocation) (.z _relativelocation)) false false)
      (else
        (Transformation|SetRelativeLocation (Variables|Default|GetTrigger) (Math|Vector|MakeVector (* (.x _relativelocation_2) (Variables|NewRoom|GetDoorPosition)) (.y _relativelocation_2) (.z _relativelocation_2)) false false)))))

(event Custom|NormalDoor
  (params (Player :type BP%20Player%20Object%20Reference))
  (if (Variables|/Game/Blueprint/Game/Player/BP_Player.BP_Player_C|GetCloseDoor Player)
    (Variables|/Game/Blueprint/Game/Player/BP_Player.BP_Player_C|SetCloseDoor Player false)
    (if (Variables|NewRoom|GetNewRoom)
      (if (not (Variables|NewRoom|GetAlreadyInNewRoom))
        (Variables|NewRoom|SetNewRoom false)
        (CallFunction|InNewRoom))
      (elif (not (Variables|NewRoom|GetNewDoor))
        (CallFunction|EventClose)))))

(event Custom|END
  (bind _outactors (Actor|GetAllActorsOfClass "/Game/Blueprint/Game/Photography/BP_Photography_END.BP_Photography_END_C"))
  (for _array_element _outactors
    (bind _asbp_photography_end (Utilities|Casting|CastToBP_Photography_END _array_element))
    (Pawn|Possess (Game|GetPlayerController 0) _asbp_photography_end)
    (Variables|/Game/Blueprint/Game/Photography/BP_Photography_END.BP_Photography_END_C|SetEND _asbp_photography_end true)))

(event EventBeginPlay
  (CallFunction|Start)
  (CallFunction|Position)
  (CallFunction|FixDoor)
  (CallFunction|Keys))

(event EventTick
  (params (DeltaSeconds :type Float%20%28single-precision%29))
  (CallFunction|KeyText)
  (if (Variables|NewRoom|GetAlreadyInNewRoom)
    (Variables|NewRoom|SetDoorPosition 1.0)
    (else
      (Variables|NewRoom|SetDoorPosition -1.0))))

(event Custom|CallNewRoom
  (params (ActualRoom :type Integer))
  (bind _outactors (Actor|GetAllActorsOfClass "/Game/Blueprint/Game/Room/BP_RoomManager.BP_RoomManager_C"))
  (for _array_element _outactors
    (if (== (+ ActualRoom 1) (Variables|/Game/Blueprint/Game/Room/BP_RoomManager.BP_RoomManager_C|GetRoom_ID _array_element))
      (Default|CallRoom _array_element)
      (Utilities|FlowControl|Delay 0.2)
      (bind _outactors_2 (Actor|GetAllActorsOfClass "/Game/Blueprint/Game/Interactable/BP_Interact.BP_Interact_C"))
      (for _array_element_2 _outactors_2
        (bind _asbp_interact (Utilities|Casting|CastToBP_Interact _array_element_2))
        (Default|UpdatePhotoPosition _asbp_interact _asbp_interact)))))

(event Custom|DestroyOldRoom
  (params (ActualRoom :type Integer))
  (bind _outactors (Actor|GetAllActorsOfClass "/Game/Blueprint/Game/Room/BP_RoomManager.BP_RoomManager_C"))
  (for _array_element _outactors
    (if (== (- ActualRoom 1) (Variables|/Game/Blueprint/Game/Room/BP_RoomManager.BP_RoomManager_C|GetRoom_ID _array_element))
      (if (not (Variables|/Game/Blueprint/Game/Room/BP_RoomManager.BP_RoomManager_C|GetClone _array_element))
        (Default|DestroyRoom _array_element)))))

(event Custom|EventOpen
  (params (ActualRoom :type Integer))
  (if (Class|KismetMathLibrary|XORBoolean (Variables|Events|GetOpen) (Variables|Events|GetAlreadyOpen))
    (CallFunction|CallNewRoom ActualRoom)
    (Variables|Events|SetDontOpenAgain true)
    (bind _newtrack_0 (Timeline|Timeline_1 PlayFromStart)
      (:Update
        (Transformation|SetRelativeRotation (Variables|Default|GetStaticMesh) (Math|Rotator|MakeRotator 0.0 0.0 (* _newtrack_0 9e+01)) false false))
      (:Finished
        (Variables|Events|SetAlreadyOpen true)
        (Components|DestroyComponent (Variables|Default|GetTextRender))
        (Variables|Default|SetInteractText 0)))))

(event Custom|EventClose
  (if (not (Variables|Events|GetBlocked))
    (bind _newtrack_0 (Timeline|Timeline_2 ReverseFromEnd)
      (:Update
        (Transformation|SetRelativeRotation (Variables|Default|GetStaticMesh) (Math|Rotator|MakeRotator 0.0 0.0 (* _newtrack_0 9e+01)) false false))
      (:Finished
        (Variables|Events|SetBlocked true)
        (Audio|PlaySound2D "/Game/Assets/StarterContent/Audio/Explosion01.Explosion01" 1.0 1.0 0.0 0 0)))))

(event Custom|InNewRoom
  (bind _trigger (Variables|Default|GetTrigger))
  (bind _relativelocation (Variables|/Script/Engine.SceneComponent|GetRelativeLocation _trigger))
  (Variables|NewRoom|SetAlreadyInNewRoom true)
  (Transformation|SetRelativeLocation (Variables|Default|GetTrigger) (Math|Vector|MakeVector (* (.x _relativelocation) (Variables|NewRoom|GetDoorPosition)) (.y _relativelocation) (.z _relativelocation)) false false)
  (bind _newtrack_0 (Timeline|Timeline_4 ReverseFromEnd)
    (:Update
      (Transformation|SetRelativeRotation (Variables|Default|GetStaticMesh) (Math|Rotator|MakeRotator 0.0 0.0 (* _newtrack_0 -9e+01)) false false))
    (:Finished
      (Audio|PlaySound2D "/Game/Assets/StarterContent/Audio/Explosion01.Explosion01" 1.0 1.0 0.0 0 0)
      (Variables|NewRoom|SetNewDoor false)
      (CallFunction|DestroyOldRoom (Variables|Default|GetID)))))

(event Custom|KeyText
  (if (!= (Variables|Default|GetID) 5)
    (if (>= (Variables|Events|GetKeyAct) (Variables|Events|GetKeyNeed))
      (if (not (Variables|Default|Getkcyo))
        (Variables|Default|Setkcyo true)
        (Rendering|Components|TextRender|SetText (Variables|Default|GetTextRender) (Variables|Default|GetOpenText))
        (Variables|Events|SetOpen true)
        (bind _asbp_gi (Utilities|Casting|CastToBP_GI (Game|GetGameInstance)))
        (Default|ShowDoorText _asbp_gi))
      (else
        (Rendering|Components|TextRender|SetText (Variables|Default|GetTextRender) (Utilities|Text|ToText(String) (Utilities|String|Append "Keys " (Utilities|String|ToString(Integer) (Variables|Events|GetKeyAct)) "/" (Utilities|String|ToString(Integer) (Variables|Events|GetKeyNeed)))))))))

(event Custom|Keys
  (bind _outactors (Actor|GetAllActorsOfClass "/Game/Blueprint/Game/Door/BP_Key.BP_Key_C"))
  (for _array_element _outactors
    (bind _asbp_key (Utilities|Casting|CastToBP_Key _array_element))
    (if (== (Variables|/Game/Blueprint/Game/Interactable/BP_Interact.BP_Interact_C|GetID _asbp_key) (Variables|Default|GetID))
      (Variables|Events|SetKeyNeed (+ (Variables|Events|GetKeyNeed) 1)))))

(fn ConstructionScript)