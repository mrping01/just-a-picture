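; Base interactable for photographs, doors and keys, branching on casts of self to those child Blueprints for setup and interaction.
; Photographs lerp by timeline to and from the player's camera, toggling their own camera and the player's spotlight.
; Doors open by ID, while keys increment the matching door's key count, destroy themselves and show key text through the game instance.
; Tick turns the prompt text toward the player or photo-capture view, gated by usability and area/use state.
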(event EventBeginPlay
  (bind _asbp_photography (Utilities|Casting|CastToBP_Photography self)
    (:then
      (CallFunction|BeginPlayPhoto _asbp_photography _asbp_photography))
    (:CastFailed
      (bind _asbp_door (Utilities|Casting|CastToBP_Door self)
        (:then
          (CallFunction|BeginPlayDoor _asbp_door _asbp_door))
        (:CastFailed
          (bind _asbp_key (Utilities|Casting|CastToBP_Key self))
          (CallFunction|BeginPlayKey _asbp_key _asbp_key))))))

(event EventTick
  (params (DeltaSeconds :type Float%20%28single-precision%29))
  (bind _interacttext (Variables|Actors|GetInteractText))
  (if (!= 0 _interacttext)
    (CallFunction|ShowText _interacttext)))

(event Custom|Interact
  (params (Player :type Actor%20Object%20Reference))
  (if (Variables|Events|GetCanUse)
    (Utilities|Casting|CastToBP_Player Player
      (:then
        ;[0.4656 0.3575 1] Actor Photography
        (bind _asbp_photography (Utilities|Casting|CastToBP_Photography self)
          (:then
            (if (Variables|BP_Interact_C|GetInUse _asbp_photography)
              (Variables|BP_Interact_C|SetCanUse _asbp_photography false)
              (CallFunction|Focus _asbp_photography Player)
              (bind _asbp_player (Utilities|Casting|CastToBP_Player Player))
              (Variables|/Game/Blueprint/Game/Player/BP_Player.BP_Player_C|SetIn%20Photo _asbp_player true)
              (Rendering|SetVisibility (Variables|/Game/Blueprint/Game/Player/BP_Player.BP_Player_C|GetSpotLight _asbp_player) false false)
              (Rendering|Components|Light|SetIntensity (Variables|/Game/Blueprint/Game/Player/BP_Player.BP_Player_C|GetSpotLight _asbp_player) 0.0)
              (else
                (Variables|BP_Interact_C|SetCanUse _asbp_photography false)
                (CallFunction|UnFocus _asbp_photography Player)
                (bind _asbp_player_2 (Utilities|Casting|CastToBP_Player Player))
                (Rendering|SetVisibility (Variables|/Game/Blueprint/Game/Player/BP_Player.BP_Player_C|GetSpotLight _asbp_player_2) true false)
                (bind _light (Timeline|Timeline PlayFromStart)
                  (:Update
                    (Rendering|Components|Light|SetIntensity (Variables|/Game/Blueprint/Game/Player/BP_Player.BP_Player_C|GetSpotLight _asbp_player) (Math|Float|Lerp (Variables|/Script/Engine.LightComponentBase|GetIntensity (Variables|/Game/Blueprint/Game/Player/BP_Player.BP_Player_C|GetSpotLight _asbp_player)) 1e+02 _light)))
                  (:Finished
                    (Variables|/Game/Blueprint/Game/Player/BP_Player.BP_Player_C|SetIn%20Photo _asbp_player_2 false))))))
          (:CastFailed
            ;[1 0.3401 0.4704] Actor Door
            (bind _asbp_door (Utilities|Casting|CastToBP_Door self)
              (:then
                (if (not (Variables|/Game/Blueprint/Game/Door/BP_Door.BP_Door_C|GetDontOpenAgain _asbp_door))
                  (Default|EventOpen _asbp_door (Variables|BP_Interact_C|GetID _asbp_door))
                  (Variables|BP_Interact_C|SetInUse _asbp_door false)))
              (:CastFailed
                ;[0.9862 1 0.3707] Actor Key
                (bind _asbp_key (Utilities|Casting|CastToBP_Key self :!label _label))
                (CallFunction|GrabKey _asbp_key))))))
      (:CastFailed
        (goto _label)))))

(event Custom|Focus
  (params (Player%20Reference :type Actor%20Object%20Reference))
  (bind _asbp_player (Utilities|Casting|CastToBP_Player Player%20Reference))
  (bind _newtrack_0 (Timeline|Timeline_Door PlayFromStart)
    (:Update
      (Transformation|SetActorTransform (Math|Transform|Lerp(Transform) (Variables|Actors|GetStartTransform) (Math|Transform|MakeTransform (+ (Transformation|GetWorldLocation (Variables|/Game/Blueprint/Game/Player/BP_Player.BP_Player_C|GetCamera _asbp_player)) (* (Math|Vector|GetForwardVector (Variables|/Game/Blueprint/Game/Player/BP_Player.BP_Player_C|GetCamera _asbp_player)) 31.0)) (Math|Rotator|MakeRotator (.roll (Transformation|GetWorldRotation (Variables|/Game/Blueprint/Game/Player/BP_Player.BP_Player_C|GetCamera _asbp_player))) (* (.pitch (Transformation|GetWorldRotation (Variables|/Game/Blueprint/Game/Player/BP_Player.BP_Player_C|GetCamera _asbp_player))) -1.0) (+ (.yaw (Transformation|GetWorldRotation (Variables|/Game/Blueprint/Game/Player/BP_Player.BP_Player_C|GetCamera _asbp_player))) 1.8e+02)) "1.500000,1.500000,1.500000") _newtrack_0)))
    (:Finished
      (bind _asbp_photography (Utilities|Casting|CastToBP_Photography self))
      (Default|ActivateCamera _asbp_photography)
      (Variables|BP_Interact_C|SetCanUse _asbp_photography true))))

(event Custom|BeginPlay%20Photo
  (params (Actor :type BP%20Photography%20Object%20Reference))
  (Variables|Actors|SetInteractText (Variables|/Game/Blueprint/Game/Photography/BP_Photography.BP_Photography_C|GetTextRender Actor))
  (Variables|Actors|SetStartTransform (Transformation|GetActorTransform Actor)))

(event Custom|UpdatePhotoPosition
  (params (Actor :type Actor%20Object%20Reference))
  (Variables|Actors|SetStartTransform (Transformation|GetActorTransform Actor)))

(event Custom|UnFocus
  (params (Player%20Reference :type Actor%20Object%20Reference))
  (bind _asbp_photography (Utilities|Casting|CastToBP_Photography self))
  (Default|ActivateCamera _asbp_photography)
  (bind _asbp_player (Utilities|Casting|CastToBP_Player Player%20Reference))
  (bind _newtrack_0 (Timeline|Timeline_0 PlayFromStart)
    (:Update
      (Transformation|SetActorTransform (Math|Transform|Lerp(Transform) (Math|Transform|MakeTransform (+ (Transformation|GetWorldLocation (Variables|/Game/Blueprint/Game/Player/BP_Player.BP_Player_C|GetCamera _asbp_player)) (* (Math|Vector|GetForwardVector (Variables|/Game/Blueprint/Game/Player/BP_Player.BP_Player_C|GetCamera _asbp_player)) 31.0)) (Math|Rotator|MakeRotator (.roll (Transformation|GetWorldRotation (Variables|/Game/Blueprint/Game/Player/BP_Player.BP_Player_C|GetCamera _asbp_player))) (* (.pitch (Transformation|GetWorldRotation (Variables|/Game/Blueprint/Game/Player/BP_Player.BP_Player_C|GetCamera _asbp_player))) -1.0) (+ (.yaw (Transformation|GetWorldRotation (Variables|/Game/Blueprint/Game/Player/BP_Player.BP_Player_C|GetCamera _asbp_player))) 1.8e+02)) "1.500000,1.500000,1.500000") (Variables|Actors|GetStartTransform) _newtrack_0)))
    (:Finished
      (bind _asbp_photography_2 (Utilities|Casting|CastToBP_Photography self))
      (Variables|BP_Interact_C|SetCanUse _asbp_photography_2 true))))

(event Custom|ShowText
  (params (Text :type Scene%20Component%20Object%20Reference))
  (if (Variables|Events|GetCanUse)
    (if (Class|KismetMathLibrary|XORBoolean (Variables|Events|GetInArea) (Variables|Events|GetInUse))
      (Rendering|SetVisibility Text true false)
      (bind _asbp_player (Utilities|Casting|CastToBP_Player (Variables|Actors|GetPlayer))
        (:then
          (Transformation|SetWorldRotation Text (Math|Rotator|MakeRotator (.roll (Math|Conversions|RotationFromXVector (Math|Vector|GetForwardVector (Variables|/Game/Blueprint/Game/Player/BP_Player.BP_Player_C|GetCamera _asbp_player)))) (* (.pitch (Math|Conversions|RotationFromXVector (Math|Vector|GetForwardVector (Variables|/Game/Blueprint/Game/Player/BP_Player.BP_Player_C|GetCamera _asbp_player)))) -1.0) (+ (.yaw (Math|Conversions|RotationFromXVector (Math|Vector|GetForwardVector (Variables|/Game/Blueprint/Game/Player/BP_Player.BP_Player_C|GetCamera _asbp_player)))) 1.8e+02)) false false))
        (:CastFailed
          (bind _asbp_player_photo (Utilities|Casting|CastToBP_PlayerPhoto (Variables|Actors|GetPlayer)))
          (Transformation|SetWorldRotation Text (Math|Rotator|MakeRotator (.roll (Math|Conversions|RotationFromXVector (Math|Vector|GetForwardVector (Variables|/Game/Blueprint/Game/Player/BP_PlayerPhoto.BP_PlayerPhoto_C|GetSceneCaptureComponent2D _asbp_player_photo)))) (* (.pitch (Math|Conversions|RotationFromXVector (Math|Vector|GetForwardVector (Variables|/Game/Blueprint/Game/Player/BP_PlayerPhoto.BP_PlayerPhoto_C|GetSceneCaptureComponent2D _asbp_player_photo)))) -1.0) (+ (.yaw (Math|Conversions|RotationFromXVector (Math|Vector|GetForwardVector (Variables|/Game/Blueprint/Game/Player/BP_PlayerPhoto.BP_PlayerPhoto_C|GetSceneCaptureComponent2D _asbp_player_photo)))) 1.8e+02)) false false)))
      (else
        (Rendering|SetVisibility Text false false :!label _label)))
    (else
      (goto _label))))

(event Custom|BeginPlay%20Door
  (params (Actor :type BP%20Door%20Object%20Reference))
  (Variables|Actors|SetInteractText (Variables|/Game/Blueprint/Game/Door/BP_Door.BP_Door_C|GetTextRender Actor))
  (Components|Timeline|SetPlayRate (Variables|BP_Interact_C|GetTimeline_Door Actor) (Variables|/Game/Blueprint/Game/Door/BP_Door.BP_Door_C|GetOpenVel Actor)))

(event Custom|BeginPlay%20Key
  (params (Actor :type BP%20Key%20Object%20Reference))
  (Variables|Actors|SetInteractText (Variables|/Game/Blueprint/Game/Door/BP_Key.BP_Key_C|GetTextRender Actor)))

(event Custom|GrabKey
  (bind _outactors (Actor|GetAllActorsOfClass "/Game/Blueprint/Game/Door/BP_Door.BP_Door_C"))
  (for _array_element _outactors
    (bind _asbp_door (Utilities|Casting|CastToBP_Door _array_element))
    (if (== (Variables|Actors|GetID) (Variables|BP_Interact_C|GetID _asbp_door))
      (Variables|/Game/Blueprint/Game/Door/BP_Door.BP_Door_C|SetKeyAct _asbp_door (+ (Variables|/Game/Blueprint/Game/Door/BP_Door.BP_Door_C|GetKeyAct _asbp_door) 1))
      (Actor|DestroyActor)
      (bind _asbp_gi (Utilities|Casting|CastToBP_GI (Game|GetGameInstance)))
      (Default|ShowKeyText _asbp_gi))))

(fn ConstructionScript)