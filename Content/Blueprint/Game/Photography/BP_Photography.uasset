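; BP_Photography is a photography prop with a point light and a photo surface that hands camera control to the BP_PlayerPhoto matching its ID.
; When in use, ActivateCamera whitens and dims the light, loops all BP_PlayerPhoto actors to set Controlling, and shows the photography material on a match.
; Otherwise it restores brighter yellow light, blacks out the photo, and releases only the loop's current element, without iterating.
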(event Custom|Activate%20Camera
  (if (Variables|Default|GetInUse)
    (Rendering|Components|Light|SetLightColor (Variables|Default|GetPointLight) (Variables|Default|GetWhiteLight) true)
    (Rendering|Components|Light|SetIntensity (Variables|Default|GetPointLight) 2.0)
    (bind _outactors (Actor|GetAllActorsOfClass "/Game/Blueprint/Game/Player/BP_PlayerPhoto.BP_PlayerPhoto_C"))
    (for _array_element _outactors
      (if (== (Variables|Default|GetID) (Variables|/Game/Blueprint/Game/Player/BP_PlayerPhoto.BP_PlayerPhoto_C|GetID _array_element))
        (Variables|/Game/Blueprint/Game/Player/BP_PlayerPhoto.BP_PlayerPhoto_C|SetControlling _array_element true)
        (Default|ActivateCamera _array_element)
        (Rendering|Material|SetMaterial (Variables|Default|GetPhoto) 0 "/Game/Blueprint/Game/Photography/MT_Photography.MT_Photography")
        (else
          (Variables|/Game/Blueprint/Game/Player/BP_PlayerPhoto.BP_PlayerPhoto_C|SetControlling _array_element false)
          (Default|ActivateCamera _array_element))))
    (else
      (Rendering|Components|Light|SetLightColor (Variables|Default|GetPointLight) (Variables|Default|GetYellowLight) true)
      (Rendering|Components|Light|SetIntensity (Variables|Default|GetPointLight) 1e+01)
      (Rendering|Material|SetMaterial (Variables|Default|GetPhoto) 0 "/Game/Blueprint/Game/Photography/MT_Black.MT_Black")
      (Variables|/Game/Blueprint/Game/Player/BP_PlayerPhoto.BP_PlayerPhoto_C|SetControlling _array_element false)
      (Default|ActivateCamera _array_element))))

(fn ConstructionScript)