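; BP_Photography_END is a photography actor that plays a closing sequence and returns to LVL_Menu.
; While its END flag is set, Tick repeatedly marks each BP_Player as ended, swaps the Photo material to MT_Photography_END and removes all widgets.
; A one-shot guarded Timeline raises the Camera by an accumulating Z offset, then opens the menu level.
; Pressing Escape opens the menu immediately.
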(event Custom|StartAnimation
  (bind _outactors (Actor|GetAllActorsOfClass "/Game/Blueprint/Game/Player/BP_Player.BP_Player_C"))
  (for _array_element _outactors
    (bind _asbp_player (Utilities|Casting|CastToBP_Player _array_element))
    (Variables|/Game/Blueprint/Game/Player/BP_Player.BP_Player_C|SetEnd _asbp_player true)
    (Rendering|Material|SetMaterial (Variables|Default|GetPhoto) 0 "/Game/Blueprint/Game/Photography/MT_Photography_END.MT_Photography_END")
    (CallFunction|Animation)
    (Viewport|RemoveAllWidgets)))

(event Custom|Animation
  (bind _camera (Variables|Default|GetCamera))
  (bind _relativelocation (Variables|/Script/Engine.SceneComponent|GetRelativeLocation _camera))
  (if (not (Variables|Default|GetAlready))
    (Variables|Default|SetAlready true)
    (bind _time (Timeline|Timeline PlayFromStart)
      (:Update
        (Transformation|SetRelativeLocation (Variables|Default|GetCamera) (Math|Vector|MakeVector (.x _relativelocation) (.y _relativelocation) (+ (* _time 5.0) (.z _relativelocation))) false false))
      (:Finished
        (Game|OpenLevel(byName) "LVL_Menu")))))

(event EventTick
  (params (DeltaSeconds :type Float%20%28single-precision%29))
  (if (Variables|Default|GetEND)
    (CallFunction|StartAnimation)))

(event Input|KeyboardEvents|Escape
  (params (Key :type Key%20Structure :default "None"))
  (:Pressed
    (Game|OpenLevel(byName) "LVL_Menu")))

(fn ConstructionScript)