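; BP_Player is the player pawn, handling mouse look, movement, interaction, UI and the pause menu.
; When InPhoto is set, it swaps body mesh and forwards movement, look and left-click interaction to a second BP_PlayerPhoto pawn with a scene capture.
; Box overlaps track the current BP_Interact, which left click activates and E releases.
; Tick drives the camera and mesh, and retargets its scene capture to the ending photo texture once End is set.
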(event Custom|Start
  (Rendering|SetVisibility (Variables|Default|GetBody) false false)
  (CallFunction|Widgets))

(event Custom|Widgets
  ;[1 1 1] UI
  (bind _returnvalue (UserInterface|CreateWidget "/Game/Blueprint/Game/UI/BP_UI.BP_UI_C"))
  (bind _output_get (Variables|Actors|SetUI _returnvalue))
  (UserInterface|Viewport|AddtoViewport _output_get 0)
  ;[1 1 1] Pause
  (bind _returnvalue_2 (UserInterface|CreateWidget "/Game/Blueprint/Game/UI/Pause/BP_Pause.BP_Pause_C"))
  (Variables|Actors|SetPause _returnvalue_2))

(event Custom|EndAnimation
  (if (Variables|Events|GetEnd)
    (Variables|/Script/Engine.SceneCaptureComponent2D|SetTextureTarget (Variables|Default|GetSceneCaptureComponent2D) "/Game/Blueprint/Game/Photography/RT_Photography_END.RT_Photography_END")))

(event EventBeginPlay
  (Pawn|Possess (Game|GetPlayerController 0) self)
  (bind _outactors (Actor|GetAllActorsOfClass "/Game/Blueprint/Game/Photography/BP_Photography_END.BP_Photography_END_C"))
  (for _array_element _outactors
    (Variables|/Game/Blueprint/Game/Photography/BP_Photography_END.BP_Photography_END_C|SetPlayer _array_element self)))

(event EventTick
  (params (DeltaSeconds :type Float%20%28single-precision%29))
  (Variables|Control|SetDelta%20Seconds DeltaSeconds)
  (Transformation|SetActorRotation (Math|Rotator|MakeRotator 0.0 0.0 (.yaw (Transformation|GetActorRotation))))
  (CallFunction|MoveCamera)
  (CallFunction|ChangeMesh)
  (CallFunction|EndAnimation))

(event Custom|VerticalMovement
  (params (Value :type Float%20%28single-precision%29))
  (if (not (Variables|Events|GetInPause))
    (if (Variables|Events|GetGameStarted)
      (if (Variables|Events|GetIn%20Photo)
        (bind _asbp_player_photo (Utilities|Casting|CastToBP_PlayerPhoto (Variables|Actors|GetNewPlayer)))
        (if (Variables|/Game/Blueprint/Game/Player/BP_PlayerPhoto.BP_PlayerPhoto_C|GetAlready _asbp_player_photo)
          (Default|VerticalMovement _asbp_player_photo Value (Variables|Control|GetVelocity)))
        (else
          (Pawn|Input|AddMovementInput (Math|Vector|GetForwardVector (Math|Rotator|MakeRotator 0.0 0.0 (.yaw (Transformation|GetActorRotation)))) Value false)
          (Variables|/Script/Engine.FloatingPawnMovement|SetMaxSpeed (Variables|Default|GetFloatingPawnMovement) (Variables|Control|GetVelocity)))))))

(event Custom|Horizontal%20Movement
  (params (Value :type Float%20%28single-precision%29))
  (if (not (Variables|Events|GetInPause))
    (if (Variables|Events|GetGameStarted)
      (if (Variables|Events|GetIn%20Photo)
        (bind _asbp_player_photo (Utilities|Casting|CastToBP_PlayerPhoto (Variables|Actors|GetNewPlayer)))
        (if (Variables|/Game/Blueprint/Game/Player/BP_PlayerPhoto.BP_PlayerPhoto_C|GetAlready _asbp_player_photo)
          (Default|HorizontalMovement _asbp_player_photo Value (Variables|Control|GetVelocity)))
        (else
          (Pawn|Input|AddMovementInput (Math|Vector|GetRightVector (Math|Rotator|MakeRotator 0.0 0.0 (.yaw (Transformation|GetActorRotation)))) Value false)
          (Variables|/Script/Engine.FloatingPawnMovement|SetMaxSpeed (Variables|Default|GetFloatingPawnMovement) (Variables|Control|GetVelocity)))))))

(event Input|AxisEvents|InputAxisVertical
  (params (AxisValue :type Float%20%28single-precision%29))
  (CallFunction|VerticalMovement AxisValue))

(event Input|AxisEvents|InputAxisHorizontal
  (params (AxisValue :type Float%20%28single-precision%29))
  (CallFunction|HorizontalMovement AxisValue))

(event OnComponentBeginOverlap(Box)
  (params (OverlappedComponent :type Primitive%20Component%20Object%20Reference) (OtherActor :type Actor%20Object%20Reference) (OtherComp :type Primitive%20Component%20Object%20Reference) (OtherBodyIndex :type Integer) (bFromSweep :type Boolean) (SweepResult :type Hit%20Result%20Structure%20%28by%20ref%29))
  (bind _asbp_interact (Utilities|Casting|CastToBP_Interact OtherActor))
  (Variables|/Game/Blueprint/Game/Interactable/BP_Interact.BP_Interact_C|SetInArea _asbp_interact true)
  (Variables|/Game/Blueprint/Game/Interactable/BP_Interact.BP_Interact_C|SetPlayer _asbp_interact self)
  (Variables|Actors|SetItemTag _asbp_interact))

(event OnComponentEndOverlap(Box)
  (params (OverlappedComponent :type Primitive%20Component%20Object%20Reference) (OtherActor :type Actor%20Object%20Reference) (OtherComp :type Primitive%20Component%20Object%20Reference) (OtherBodyIndex :type Integer))
  (bind _asbp_interact (Utilities|Casting|CastToBP_Interact OtherActor))
  (Variables|/Game/Blueprint/Game/Interactable/BP_Interact.BP_Interact_C|SetInArea _asbp_interact false)
  (Variables|Actors|SetItemTag 0))

(event OnComponentBeginOverlap(Body)
  (params (OverlappedComponent :type Primitive%20Component%20Object%20Reference) (OtherActor :type Actor%20Object%20Reference) (OtherComp :type Primitive%20Component%20Object%20Reference) (OtherBodyIndex :type Integer) (bFromSweep :type Boolean) (SweepResult :type Hit%20Result%20Structure%20%28by%20ref%29))
  (Utilities|Casting|CastToBP_Door OtherActor)
  (Variables|Actors|SetCloseDoor true))

(event Custom|Change%20Mesh
  (if (Variables|Events|GetIn%20Photo)
    (if (!= "/Game/Assets/StarterContent/Shapes/Shape_NarrowCapsule.Shape_NarrowCapsule" (Variables|Default|GetBody))
      (Components|StaticMesh|SetStaticMesh (Variables|Default|GetBody) "/Game/Assets/StarterContent/Shapes/Shape_NarrowCapsule.Shape_NarrowCapsule"))
    (elif (!= "/Game/Assets/StarterContent/Shapes/SM_Capsule_Modified.SM_Capsule_Modified" (Variables|Default|GetBody))
      (Components|StaticMesh|SetStaticMesh (Variables|Default|GetBody) "/Game/Assets/StarterContent/Shapes/SM_Capsule_Modified.SM_Capsule_Modified"))))

(event Input|MouseEvents|LeftMouseButton
  (params (Key :type Key%20Structure))
  (:Pressed
    (if (not (Variables|Events|GetInPause))
      (if (Variables|Events|GetIn%20Photo)
        (bind _asbp_player_photo (Utilities|Casting|CastToBP_PlayerPhoto (Variables|Actors|GetNewPlayer)))
        (bind _asbp_interact (Utilities|Casting|CastToBP_Interact (Variables|/Game/Blueprint/Game/Player/BP_PlayerPhoto.BP_PlayerPhoto_C|GetItemTag _asbp_player_photo)))
        (if (not (Variables|/Game/Blueprint/Game/Interactable/BP_Interact.BP_Interact_C|GetInUse _asbp_interact))
          (Variables|/Game/Blueprint/Game/Interactable/BP_Interact.BP_Interact_C|SetInUse _asbp_interact true)
          (Default|Interact _asbp_interact _asbp_player_photo))
        (else
          (bind _asbp_interact_2 (Utilities|Casting|CastToBP_Interact (Variables|Actors|GetItemTag)))
          (if (not (Variables|/Game/Blueprint/Game/Interactable/BP_Interact.BP_Interact_C|GetInUse _asbp_interact_2))
            (Variables|/Game/Blueprint/Game/Interactable/BP_Interact.BP_Interact_C|SetInUse _asbp_interact_2 true)
            (Default|Interact _asbp_interact_2 self)))))))

(event Input|KeyboardEvents|E
  (params (Key :type Key%20Structure))
  (:Pressed
    (bind _asbp_interact (Utilities|Casting|CastToBP_Interact (Variables|Actors|GetItemTag)))
    (if (Variables|/Game/Blueprint/Game/Interactable/BP_Interact.BP_Interact_C|GetInUse _asbp_interact)
      (Variables|/Game/Blueprint/Game/Interactable/BP_Interact.BP_Interact_C|SetInUse _asbp_interact false)
      (Default|Interact _asbp_interact self))))

(event Custom|Move%20Camera
  (if (not (Variables|Events|GetInPause))
    (if (Variables|Events|GetGameStarted)
      (bind _asbp_gi (Utilities|Casting|CastToBP_GI (Game|GetGameInstance)))
      (if (Variables|Events|GetIn%20Photo)
        (bind _asbp_player_photo (Utilities|Casting|CastToBP_PlayerPhoto (Variables|Actors|GetNewPlayer)))
        (Transformation|SetRelativeRotation (Variables|/Game/Blueprint/Game/Player/BP_PlayerPhoto.BP_PlayerPhoto_C|GetBody _asbp_player_photo) (Math|Rotator|MakeRotator 0.0 0.0 (.NewPosX (Utilities|CameraCalculates (.pitch (Variables|/Script/Engine.SceneComponent|GetRelativeRotation (Variables|/Game/Blueprint/Game/Player/BP_PlayerPhoto.BP_PlayerPhoto_C|GetSceneCaptureComponent2D _asbp_player_photo))) (Input|AxisValues|GetLookUp/DownMouse) (Variables|/Game/Map/Game/BP_GI.BP_GI_C|GetMouseSens _asbp_gi) (Input|AxisValues|GetTurnRight/LeftMouse) (.yaw (Variables|/Script/Engine.SceneComponent|GetRelativeRotation (Variables|/Game/Blueprint/Game/Player/BP_PlayerPhoto.BP_PlayerPhoto_C|GetBody _asbp_player_photo)))))) false false)
        (Transformation|SetRelativeRotation (Variables|/Game/Blueprint/Game/Player/BP_PlayerPhoto.BP_PlayerPhoto_C|GetSceneCaptureComponent2D _asbp_player_photo) (Math|Rotator|MakeRotator 0.0 (.NewPosY (Utilities|CameraCalculates (.pitch (Variables|/Script/Engine.SceneComponent|GetRelativeRotation (Variables|/Game/Blueprint/Game/Player/BP_PlayerPhoto.BP_PlayerPhoto_C|GetSceneCaptureComponent2D _asbp_player_photo))) (Input|AxisValues|GetLookUp/DownMouse) (Variables|/Game/Map/Game/BP_GI.BP_GI_C|GetMouseSens _asbp_gi) (Input|AxisValues|GetTurnRight/LeftMouse) (.yaw (Variables|/Script/Engine.SceneComponent|GetRelativeRotation (Variables|/Game/Blueprint/Game/Player/BP_PlayerPhoto.BP_PlayerPhoto_C|GetBody _asbp_player_photo))))) 0.0) false false)
        (else
          (Transformation|SetRelativeRotation (Variables|Default|GetCamera) (Math|Rotator|MakeRotator 0.0 (.NewPosY (Utilities|CameraCalculates (.pitch (Variables|/Script/Engine.SceneComponent|GetRelativeRotation (Variables|Default|GetCamera))) (Input|AxisValues|GetLookUp/DownMouse) (Variables|/Game/Map/Game/BP_GI.BP_GI_C|GetMouseSens _asbp_gi) (Input|AxisValues|GetTurnRight/LeftMouse) (.yaw (Variables|/Script/Engine.SceneComponent|GetRelativeRotation (Variables|Default|GetBody))))) 0.0) false false)
          (Transformation|SetRelativeRotation (Variables|Default|GetBody) (Math|Rotator|MakeRotator 0.0 0.0 (.NewPosX (Utilities|CameraCalculates (.pitch (Variables|/Script/Engine.SceneComponent|GetRelativeRotation (Variables|Default|GetCamera))) (Input|AxisValues|GetLookUp/DownMouse) (Variables|/Game/Map/Game/BP_GI.BP_GI_C|GetMouseSens _asbp_gi) (Input|AxisValues|GetTurnRight/LeftMouse) (.yaw (Variables|/Script/Engine.SceneComponent|GetRelativeRotation (Variables|Default|GetBody)))))) false false))))))

(event Custom|PauseEvent
  (bind _returnvalue (Game|GetPlayerController 0))
  (bind _returnvalue_2 (Game|GetPlayerController 0))
  (bind _pause (Variables|Actors|GetPause))
  (if (Variables|Events|GetInPause)
    (Variables|Events|SetInPause false)
    (Viewport|RemoveAllWidgets)
    (UserInterface|Viewport|AddtoViewport (Variables|Actors|GetUI) 0)
    (Variables|/Script/Engine.PlayerController|SetbShowMouseCursor _returnvalue false)
    (Input|SetInputModeGameOnly _returnvalue false)
    (else
      (Variables|Events|SetInPause true)
      (Viewport|RemoveAllWidgets)
      (UserInterface|Viewport|AddtoViewport _pause 0)
      (Variables|/Script/Engine.PlayerController|SetbShowMouseCursor _returnvalue_2 true)
      (Input|SetInputModeGameandUI _returnvalue_2 _pause "DoNotLock" false false))))

(event Input|KeyboardEvents|Escape
  (params (Key :type Key%20Structure :default "None"))
  (:Pressed
    (if (Variables|Events|GetGameStarted)
      (CallFunction|PauseEvent))))

(fn ConstructionScript)