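; BP_PlayerPhoto is a floating player pawn whose scene capture renders to the photography render target while it is being controlled.
; ActivateCamera toggles the capture with Controlling and registers the pawn as NewPlayer on every BP_Player.
; Tick flattens rotation to yaw, swaps the body mesh by control state, and passes Controlling to BP_RoomManager's CloneRoom when room IDs match.
; It also handles yaw-relative movement and box-overlap detection of BP_Interact items.
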(event Custom|Change%20Mesh
  (if (Variables|Events|GetControlling)
    (if (!= "/Game/Assets/StarterContent/Shapes/SM_Capsule_Modified.SM_Capsule_Modified" (Variables|Default|GetBody))
      (Components|StaticMesh|SetStaticMesh (Variables|Default|GetBody) "/Game/Assets/StarterContent/Shapes/SM_Capsule_Modified.SM_Capsule_Modified"))
    (elif (!= "/Game/Assets/StarterContent/Shapes/Shape_NarrowCapsule.Shape_NarrowCapsule" (Variables|Default|GetBody))
      (Components|StaticMesh|SetStaticMesh (Variables|Default|GetBody) "/Game/Assets/StarterContent/Shapes/Shape_NarrowCapsule.Shape_NarrowCapsule"))))

(event Custom|Activate%20Camera
  (if (Variables|Events|GetControlling)
    (if (not (Variables|Events|GetAlready))
      (Variables|/Script/Engine.SceneCaptureComponent2D|SetTextureTarget (Variables|Default|GetSceneCaptureComponent2D) "/Game/Blueprint/Game/Photography/RT_Photography.RT_Photography")
      (Components|Tick|SetComponentTickEnabled (Variables|Default|GetSceneCaptureComponent2D) true)
      (Rendering|SetVisibility (Variables|Default|GetSceneCaptureComponent2D) true true)
      (Variables|Events|SetAlready true)
      (bind _outactors (Actor|GetAllActorsOfClass "/Game/Blueprint/Game/Player/BP_Player.BP_Player_C"))
      (for _array_element _outactors
        (Variables|/Game/Blueprint/Game/Player/BP_Player.BP_Player_C|SetNewPlayer _array_element self)))
    (else
      (Variables|/Script/Engine.SceneCaptureComponent2D|SetTextureTarget (Variables|Default|GetSceneCaptureComponent2D) 0)
      (Components|Tick|SetComponentTickEnabled (Variables|Default|GetSceneCaptureComponent2D) false)
      (Rendering|SetVisibility (Variables|Default|GetSceneCaptureComponent2D) false true)
      (Variables|Events|SetAlready false))))

(event Custom|RoomVisible
  (bind _returnvalue (Actor|GetActorOfClass "/Game/Blueprint/Game/Room/BP_RoomManager.BP_RoomManager_C"))
  (bind _asbp_room_manager (Utilities|Casting|CastToBP_RoomManager _returnvalue))
  (if (== (Variables|Actors|GetRoom_ID) (Variables|/Game/Blueprint/Game/Room/BP_RoomManager.BP_RoomManager_C|GetRoom_ID _asbp_room_manager))
    (Default|CloneRoom _asbp_room_manager (Variables|Events|GetControlling))))

(event EventTick
  (params (DeltaSeconds :type Float%20%28single-precision%29))
  (Transformation|SetActorRotation (Math|Rotator|MakeRotator 0.0 0.0 (.yaw (Transformation|GetActorRotation))))
  (CallFunction|ChangeMesh)
  (CallFunction|RoomVisible))

(event EventBeginPlay
  (Rendering|SetVisibility (Variables|Default|GetBody) false false))

(event Custom|Horizontal%20Movement
  (params (Axis%20Value :type Float%20%28double-precision%29) (Velocity :type Float%20%28double-precision%29))
  (Pawn|Input|AddMovementInput (Math|Vector|GetRightVector (Math|Rotator|MakeRotator 0.0 0.0 (.yaw (Transformation|GetActorRotation)))) Axis%20Value false)
  (Variables|/Script/Engine.FloatingPawnMovement|SetMaxSpeed (Variables|Default|GetFloatingPawnMovement) Velocity))

(event Custom|Vertical%20Movement
  (params (Axis%20Value :type Float%20%28double-precision%29) (Velocity :type Float%20%28double-precision%29))
  (Pawn|Input|AddMovementInput (Math|Vector|GetForwardVector (Math|Rotator|MakeRotator 0.0 0.0 (.yaw (Transformation|GetActorRotation)))) Axis%20Value false)
  (Variables|/Script/Engine.FloatingPawnMovement|SetMaxSpeed (Variables|Default|GetFloatingPawnMovement) Velocity))

(event OnComponentBeginOverlap(Box)
  (params (OverlappedComponent :type Primitive%20Component%20Object%20Reference) (OtherActor :type Actor%20Object%20Reference) (OtherComp :type Primitive%20Component%20Object%20Reference) (OtherBodyIndex :type Integer) (bFromSweep :type Boolean) (SweepResult :type Hit%20Result%20Structure%20%28by%20ref%29))
  (bind _asbp_interact (Utilities|Casting|CastToBP_Interact OtherActor))
  (Variables|/Game/Blueprint/Game/Interactable/BP_Interact.BP_Interact_C|SetInArea _asbp_interact true)
  (Variables|/Game/Blueprint/Game/Interactable/BP_Interact.BP_Interact_C|SetPlayer _asbp_interact self)
  (Variables|Actors|SetItemTag _asbp_interact))

(event OnComponentEndOverlap(Box)
  (params (OverlappedComponent :type Primitive%20Component%20Object%20Reference) (OtherActor :type Actor%20Object%20Reference) (OtherComp :type Primitive%20Component%20Object%20Reference) (OtherBodyIndex :type Integer))
  (bind _asbp_interact (Utilities|Casting|CastToBP_Interact OtherActor))
  (Variables|/Game/Blueprint/Game/Interactable/BP_Interact.BP_Interact_C|SetInArea _asbp_interact false)
  (Variables|Actors|SetItemTag 0))

(fn ConstructionScript)