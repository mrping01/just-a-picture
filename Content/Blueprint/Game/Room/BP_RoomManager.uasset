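; BP_RoomManager is a room actor that shows, hides and repositions itself and its child components according to its RoomID.
; At BeginPlay, clones pass RoomID to attached BP_PlayerPhoto actors, while non-clone rooms other than the first hide themselves.
; CallRoom reveals the room in one of two fixed slots chosen by RoomID parity.
; DestroyRoom only hides it and parks it far away, and CloneRoom just sets visibility.
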(event Custom|CallRoom
  (if (!= (Math|Integer|%(Integer) (Variables|Default|GetRoom_ID) 2) 0)
    (Transformation|SetActorLocation "0.000000,-215.000000,0.000000" false false)
    (else
      (Transformation|SetActorLocation "600.000000,-215.000000,0.000000" false false)))
  (Rendering|SetVisibility (Variables|Transformation|GetRootComponent) true true))

(event Custom|DestroyRoom
  (Transformation|SetActorLocation "4000.000000,4000.000000,4000.000000" false false)
  (Rendering|SetVisibility (Variables|Transformation|GetRootComponent) false true))

(event Custom|CloneRoom
  (params (bNewVisibility :type Boolean))
  (Rendering|SetVisibility (Variables|Transformation|GetRootComponent) bNewVisibility true))

(event EventBeginPlay
  (if (Variables|Default|GetClone)
    (for _array_element (Actor|GetAttachedActors true false)
      (bind _asbp_player_photo (Utilities|Casting|CastToBP_PlayerPhoto _array_element))
      (Variables|/Game/Blueprint/Game/Player/BP_PlayerPhoto.BP_PlayerPhoto_C|SetRoom_ID _asbp_player_photo (Variables|Default|GetRoom_ID)))
    (elif (not (== 1 (Variables|Default|GetRoom_ID)))
      (Rendering|SetVisibility (Variables|Transformation|GetRootComponent) false true))))

(fn ConstructionScript)