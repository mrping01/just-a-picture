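; BP_Menu is the possessed main menu actor that creates the menu, options and credits widgets and sets up mouse-driven UI input and windowed fullscreen.
; ChangeView clears widgets, slides the Sphere component along X by timeline, then shows options, credits or the main menu based on InOptions and Page.
; StartView plays its own slide before opening LVL_Test.
; Tick writes the current FPS to the BP_GI game instance.
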(event Custom|GetFPS
  (params (InputPin :type Float%20%28double-precision%29))
  (bind _asbp_gi (Utilities|Casting|CastToBP_GI (Game|GetGameInstance)))
  (Variables|/Game/Map/Game/BP_GI.BP_GI_C|SetFPS _asbp_gi (/ 1.0 InputPin)))

(event Custom|Start
  (Pawn|Possess (Game|GetPlayerController 0) self)
  ;[1 1 1] Menu
  (bind _returnvalue (UserInterface|CreateWidget "/Game/Blueprint/Menu/UI/BP_MainMenu_Menu.BP_MainMenu_Menu_C"))
  (bind _output_get (Variables|UI|SetUI_Menu _returnvalue))
  (UserInterface|Viewport|AddtoViewport _output_get 0)
  (Input|SetInputModeUIOnly (Game|GetPlayerController 0) _output_get "DoNotLock" false)
  ;[1 1 1] Menu
  (bind _returnvalue_2 (UserInterface|CreateWidget "/Game/Blueprint/Menu/UI/BP_MainMenu_Options.BP_MainMenu_Options_C"))
  (Variables|UI|SetUI_Options _returnvalue_2)
  ;[1 1 1] Credits
  (bind _returnvalue_3 (UserInterface|CreateWidget "/Game/Blueprint/Menu/UI/BP_MainMenu_Credits.BP_MainMenu_Credits_C"))
  (Variables|UI|SetUI_Credits _returnvalue_3)
  (Variables|/Script/Engine.PlayerController|SetbShowMouseCursor (Game|GetPlayerController 0) true)
  (bind _returnvalue_4 (Settings|GetGameUserSettings))
  (Class|GameUserSettings|SetFullscreenMode _returnvalue_4 "WindowedFullscreen"))

(event Custom|ChangeView
  (params (Page :type Integer))
  (Viewport|RemoveAllWidgets)
  (bind _movement (Timeline|Timeline PlayFromStart)
    (:Update
      (Transformation|SetRelativeLocation (Variables|Default|GetSphere) (Math|Vector|MakeVector (* _movement -4e+01) 0.0 0.0) false false))
    (:Finished
      (if (Variables|Default|GetInOptions)
        (switch int Page
          (:0
            (UserInterface|Viewport|AddtoViewport (Variables|UI|GetUI_Options) 0))
          (:1
            (UserInterface|Viewport|AddtoViewport (Variables|UI|GetUI_Credits) 0)))
        (else
          (UserInterface|Viewport|AddtoViewport (Variables|UI|GetUI_Menu) 0))))))

(event Custom|StartView
  (Viewport|RemoveAllWidgets)
  (bind _movement (Timeline|Timeline_0 PlayFromStart)
    (:Update
      (Transformation|SetRelativeLocation (Variables|Default|GetSphere) (Math|Vector|MakeVector (* _movement 55.0) 0.0 0.0) false false))
    (:Finished
      (Game|OpenLevel(byName) "LVL_Test"))))

(event EventTick
  (params (DeltaSeconds :type Float%20%28single-precision%29))
  (CallFunction|GetFPS DeltaSeconds))

(event EventBeginPlay
  (CallFunction|Start))

(fn ConstructionScript)