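; Game instance Blueprint (judging by its name) that holds transient key and door prompt flags and applies the graphics quality setting.
; The door and key text events raise their flag for a few seconds and then clear it; the door event also clears the key flag first.
; SetQuality applies one Quality index to the scalability groups, looks up resolution scale by that index, uncaps frame rate and applies the settings.
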(event Custom|SetQuality
  (bind _quality (Variables|Options|GetQuality))
  (bind _returnvalue (Settings|GetGameUserSettings))
  (Class|GameUserSettings|SetFrameRateLimit _returnvalue 0.0)
  (Class|GameUserSettings|SetAntiAliasingQuality _returnvalue _quality)
  (Class|GameUserSettings|SetAudioQualityLevel _returnvalue _quality)
  (Class|GameUserSettings|SetFoliageQuality _returnvalue _quality)
  (Class|GameUserSettings|SetGlobalIlluminationQuality _returnvalue _quality)
  (Class|GameUserSettings|SetPostProcessingQuality _returnvalue _quality)
  (Class|GameUserSettings|SetReflectionQuality _returnvalue _quality)
  (Class|GameUserSettings|SetShadingQuality _returnvalue _quality)
  (Class|GameUserSettings|SetShadowQuality _returnvalue _quality)
  (Class|GameUserSettings|SetTextureQuality _returnvalue _quality)
  (Class|GameUserSettings|SetTextureQuality _returnvalue _quality)
  (Class|GameUserSettings|SetViewDistanceQuality _returnvalue _quality)
  (Class|GameUserSettings|SetVisualEffectQuality _returnvalue _quality)
  (Class|GameUserSettings|SetResolutionScaleValueEx _returnvalue (Utilities|Array|Get(acopy) (Variables|Options|GetResolutionScale) _quality))
  (Class|GameUserSettings|ApplySettings _returnvalue true))

(event Custom|ShowKeyText
  (Variables|Events|SetKeyGrabbed true)
  (Utilities|FlowControl|Delay 2.5)
  (Variables|Events|SetKeyGrabbed false))

(event Custom|ShowDoorText
  (Variables|Events|SetKeyGrabbed false)
  (Variables|Events|SetDoorOpen true)
  (Utilities|FlowControl|Delay 3.0)
  (Variables|Events|SetDoorOpen false))